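; BP_chess is a board game piece actor that animates flipping itself over, as in a Reversi-style game.
; Its reverse event caches the Chess component's world transform, then plays a timeline that offsets the actor's height and roll from that start.
; When the timeline finishes, it decrements the Board's ReverseNum counter and clears its IsFlipping flag.
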(event Custom|reverse
  (bind _board (Variables|Default|Getboard))
  (Variables|Default|Setrotation (Transformation|GetWorldRotation (Variables|Default|Getchess)))
  (Variables|Default|Setlocation (Transformation|GetWorldLocation (Variables|Default|Getchess)))
  (bind (_direction _high _rotation) (Timeline|Timeline_reverse PlayFromStart)
    (:Update
      (Transformation|SetActorLocation (Math|Vector|MakeVector (.X (Math|Vector|BreakVector (Variables|Default|Getlocation))) (.Y (Math|Vector|BreakVector (Variables|Default|Getlocation))) (+ (.Z (Math|Vector|BreakVector (Variables|Default|Getlocation))) _high)) false false)
      (Transformation|SetActorRotation (Math|Rotator|MakeRotator (+ (.Roll (Math|Rotator|BreakRotator (Variables|Default|Getrotation))) _rotation) (.Pitch (Math|Rotator|BreakRotator (Variables|Default|Getrotation))) (.Yaw (Math|Rotator|BreakRotator (Variables|Default|Getrotation))))))
    (:Finished
      (Variables|/Script/Reversi.checkerboard|Setreverse_num _board (- (Variables|/Script/Reversi.checkerboard|Getreverse_num _board) 1))
      (Variables|Default|Setis_flipping false))))

(event EventBeginPlay)

(event Collision|EventActorBeginOverlap
  (params (OtherActor :type Actor%20Object%20Reference)))

(event EventTick
  (params (DeltaSeconds :type Float%20%28single-precision%29)))

(fn ConstructionScript)